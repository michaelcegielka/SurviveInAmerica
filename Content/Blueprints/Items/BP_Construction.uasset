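; Buildable construction site that shows a ghost-material blueprint and fills in as resources are dropped into it.
; Construction script loads required resource counts from a DT_Constructions row.
; Overlapping BP_Resource actors of a needed type decrement that count, are destroyed, and flag the slot once satisfied.
; EvolveMesh then adds a static mesh component at the next free Log or Beam socket, consuming sockets cached on BeginPlay.
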(event `self.ReceiveBeginPlay`
  (`parent.ReceiveBeginPlay`)
  (`|ExecutionSequence`
    (:`then_0`
      (for _array_element (`SceneComponent.GetAllSocketNames` (`self.StaticMesh`))
        (`KismetArrayLibrary.Array_Add` (`self.SocketsFloor`) _array_element)))
    (:`then_1`
      (for _array_element_2 (`SceneComponent.GetAllSocketNames` (`self.Beams`))
        (`KismetArrayLibrary.Array_Add` (`self.SocketsBeams`) _array_element_2)))))

(event `self.Collision.OnComponentBeginOverlap`
  (params (OverlappedComponent :type "PrimitiveComponent Object Reference") (OtherActor :type "Actor Object Reference") (OtherComp :type "PrimitiveComponent Object Reference") (OtherBodyIndex :type Integer) (bFromSweep :type Boolean) (SweepResult :type "HitResult Structure (by ref)"))
  (bind _asbp_resource (cast `/Game/Blueprints/Items/BP_Resource` OtherActor))
  (`self.AddResource` _asbp_resource))

(fn `AddResource`
  (params (ResourceToAdd :type "/Game/Blueprints/Items/BP_Resource Object Reference"))
  (locals (TMP_resource :type "/Game/Blueprints/Items/BP_Resource Object Reference") (TMP_type :type "/Game/Blueprints/ENUMs/E_ResourceType Enum"))
  (bind (_constructiondata_name _constructiondata_ressources) (break `/Game/Blueprints/Structures/STRUCT_ConstructionData` (`self.ConstructionData`)))
  (bind (_constructiondata_name_2 _constructiondata_ressources_2) (break `/Game/Blueprints/Structures/STRUCT_ConstructionData` (`self.ConstructionData`)))
  (set `local.TMP_resource` ResourceToAdd)
  (set `local.TMP_type` (`/Game/Blueprints/Items/BP_Resource.GetType` (`local.TMP_resource`)))
  (if (`BlueprintMapLibrary.Map_Contains` _constructiondata_ressources_2 (`local.TMP_type`))
    (bind _keys (`BlueprintMapLibrary.Map_Keys` _constructiondata_ressources_2))
    (for (_array_element _array_index) _keys
      (if (`|EnumEquality` (`local.TMP_type`) _array_element)
        (if (> (`BlueprintMapLibrary.Map_Find` _constructiondata_ressources_2 _array_element) 0)
          (bind _value (`BlueprintMapLibrary.Map_Find` _constructiondata_ressources _array_element))
          (`/Engine/EditorBlueprintResources/StandardMacros.DecrementInt` _value
            (:`  `
              (`self.K2_DestroyActor` (`local.TMP_resource`))
              (`self.EvolveMesh` (`local.TMP_type`))
              (set `local.TMP_resource` null)
              (set `local.TMP_type` "NewEnumerator3")
              (if (== _value 0)
                (`KismetArrayLibrary.Array_Set` (`self.ConstructionSlots`) _array_index true)))))))))

(fn `EvolveMesh`
  (params (`New Resource Type` :type "/Game/Blueprints/ENUMs/E_ResourceType Enum" :default "NewEnumerator3"))
  (locals (FoundSocket :type Boolean) (TMP_Socket :type Name))
  (bind _staticmesh (`self.StaticMesh`))
  (bind _beams (`self.Beams`))
  (switch `/Game/Blueprints/ENUMs/E_ResourceType` `New Resource Type`
    (:`NewEnumerator0`
      (`KismetSystemLibrary.PrintString` "Evolving")
      (for _array_element (`self.SocketsFloor`)
        (if (`KismetStringLibrary.StartsWith` (`KismetStringLibrary.Conv_NameToString` _array_element) "Log")
          (set `local.FoundSocket` true)
          (set `local.TMP_Socket` _array_element)
          (break)))
      (if (`local.FoundSocket`)
        (for _array_element_2 (`SceneComponent.GetAllSocketNames` _staticmesh)
          (if (== _array_element_2 (`local.TMP_Socket`))
            (bind _returnvalue (`AddComponent|NODE_AddStaticMeshComponent-0`))
            (bind _returnvalue_2 (`SceneComponent.GetSocketTransform` _staticmesh _array_element_2 "RTS_World"))
            (`SceneComponent.K2_SetWorldTransform` _returnvalue (`KismetMathLibrary.MakeTransform` (.location _returnvalue_2) (`KismetMathLibrary.MakeRotator` (+ (.roll (.rotation _returnvalue_2)) 90.0) (.pitch (.rotation _returnvalue_2)) (.yaw (.rotation _returnvalue_2))) (* (.scale _returnvalue_2) (1.1 1.1 1.1))) false false)
            (`KismetArrayLibrary.Array_RemoveItem` (`self.SocketsFloor`) _array_element_2)))))
    (:`NewEnumerator4`
      (for _array_element_3 (`self.SocketsBeams`)
        (if (`KismetStringLibrary.StartsWith` (`KismetStringLibrary.Conv_NameToString` _array_element_3) "Beam")
          (set `local.FoundSocket` true)
          (set `local.TMP_Socket` _array_element_3)
          (break)))
      (if (`local.FoundSocket`)
        (for _array_element_4 (`SceneComponent.GetAllSocketNames` _beams)
          (if (== _array_element_4 (`local.TMP_Socket`))
            (bind _returnvalue_3 (`AddComponent|NODE_AddStaticMeshComponent-1`))
            (bind _returnvalue_4 (`SceneComponent.GetSocketTransform` _beams _array_element_4 "RTS_World"))
            (`SceneComponent.K2_SetWorldTransform` _returnvalue_3 (`KismetMathLibrary.MakeTransform` (.location _returnvalue_4) (`KismetMathLibrary.MakeRotator` (.roll (.rotation _returnvalue_4)) (+ (.pitch (.rotation _returnvalue_4)) 90.0) (.yaw (.rotation _returnvalue_4))) (* (.scale _returnvalue_4) (1.1 1.1 1.1))) false false)
            (`KismetArrayLibrary.Array_RemoveItem` (`self.SocketsBeams`) _array_element_4)))))))

(fn `UserConstructionScript`
  (`parent.UserConstructionScript`)
  (`|ExecutionSequence`
    (:`then_0`
      (bind _returnvalue (`|GetDataTableRow` "/Game/Blueprints/DataTables/DT_Constructions.DT_Constructions" (`self.DT_Row`))
        (:`then`
          (set `self.ConstructionData` _returnvalue)
          (bind _keys (`BlueprintMapLibrary.Map_Keys` (`.Ressources_19_1B508FE4462461BD600E7A9F59D0B6A1` (break `/Game/Blueprints/Structures/STRUCT_ConstructionData` (`self.ConstructionData`)))))
          (for _ _keys
            (`KismetArrayLibrary.Array_Add` (`self.ConstructionSlots`))))))
    (:`then_1`
      (`PrimitiveComponent.SetMaterial` (`self.StaticMesh`) 0 "/Game/Materials/M_Ghost_Inst.M_Ghost_Inst")
      (`PrimitiveComponent.SetMaterial` (`self.StaticMesh`) 0 "/Game/Materials/M_Ghost_Inst.M_Ghost_Inst")
      (`PrimitiveComponent.SetMaterial` (`self.Beams`) 0 "/Game/Materials/M_Ghost_Inst.M_Ghost_Inst"))))