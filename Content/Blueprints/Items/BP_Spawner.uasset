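; BP_Spawner scatters copies of a chosen object at random points inside its Boundary component when play begins.
; SetSpawnpoints samples random XY positions within the boundary's bounds at a fixed height, dropping exact duplicates without retrying.
; SpawnObjects then spawns the requested number with random yaw, removing each used point so locations are not reused.
; The candidate location count is printed for debugging.
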(event `self.ReceiveBeginPlay`
  (`self.SetSpawnpoints`)
  (`KismetSystemLibrary.PrintString` (`KismetStringLibrary.Conv_IntToString` (`KismetArrayLibrary.Array_Length` (`self.SpawnLocations`))))
  (`self.SpawnObjects`))

(fn `SetSpawnpoints`
  (locals (XmaxYmax :type "Vector Structure") (XmaxYmin :type "Vector Structure") (XminYmax :type "Vector Structure") (XminYmin :type "Vector Structure") (RandomVector :type "Vector Structure" :default (0.0 0.0 0.0)) (NothingsimiliarFound :type Boolean :default true))
  (bind _spawnlocations (`self.SpawnLocations`))
  (bind (_xmaxymax_x _xmaxymax_y) (`KismetMathLibrary.BreakVector` (`local.XmaxYmax`)))
  (bind (_xminymin_x _xminymin_y) (`KismetMathLibrary.BreakVector` (`local.XminYmin`)))
  (bind (_origin _boxextent) (`KismetSystemLibrary.GetComponentBounds` (`self.Boundary`)))
  (set `local.XmaxYmax` (+ _origin (`KismetMathLibrary.MakeVector` (.x _boxextent) (.y _boxextent) 5.0)))
  (set `local.XmaxYmin` (`KismetMathLibrary.MakeVector` (+ (.x _origin) (.x _boxextent)) (- (.y _origin) (.y _boxextent)) 5.0))
  (set `local.XminYmax` (`KismetMathLibrary.MakeVector` (- (.x _origin) (.x _boxextent)) (+ (.y _origin) (.y _boxextent)) 5.0))
  (set `local.XminYmin` (- _origin (`KismetMathLibrary.MakeVector` (.x _boxextent) (.y _boxextent) 5.0)))
  (for _ (range (`self.AmountOfSpawnLocations`))
    (set `local.RandomVector` (`KismetMathLibrary.MakeVector` (`KismetMathLibrary.RandomFloatInRange` _xminymin_x _xmaxymax_x) (`KismetMathLibrary.RandomFloatInRange` _xminymin_y _xmaxymax_y) 5.0))
    (if (`KismetArrayLibrary.Array_IsNotEmpty` _spawnlocations)
      (for _array_element _spawnlocations
        (if (not (!= _array_element (`local.RandomVector`)))
          (set `local.NothingsimiliarFound` false)))
      (if (`local.NothingsimiliarFound`)
        (`KismetArrayLibrary.Array_Add` _spawnlocations (`local.RandomVector`) :!label _label)
        (set `local.NothingsimiliarFound` true)
        (else
          (set `local.NothingsimiliarFound` true)))
      (else
        (goto _label)))))

(fn `SpawnObjects`
  (locals (SpawnLocationIndex :type Integer :default 0))
  (bind _spawnlocations (`self.SpawnLocations`))
  (for _ (range (`self.AmountToSpawn`))
    (set `local.SpawnLocationIndex` (`KismetMathLibrary.RandomIntegerInRange` 0 (- (`KismetArrayLibrary.Array_Length` _spawnlocations) 1)))
    (`|SpawnActorFromClass` (`GameplayStatics.GetObjectClass` (`self.ObjectToSpawn`)) (`KismetMathLibrary.MakeTransform` (`|GetArrayItem` _spawnlocations (`local.SpawnLocationIndex`)) (`KismetMathLibrary.MakeRotator` 0.0 0.0 (`KismetMathLibrary.RandomFloatInRange` 0.0 180.0))) "Undefined" "MultiplyWithRoot" null null)
    (`KismetArrayLibrary.Array_Remove` (`self.SpawnLocations`) (`local.SpawnLocationIndex`))
    (set `local.SpawnLocationIndex` 0)))

(fn `UserConstructionScript`)