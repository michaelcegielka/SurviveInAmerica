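; BP_Resource is a data-driven resource item actor whose identity comes from a row in the DT_Resources data table.
; The construction script looks up the DTRow entry, caches it as ResourceData, and applies its mesh and grab sound to the actor.
; GetName returns the name from the cached row, and the event graph holds only disabled default events.
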(fn `GetName`
  (returns (`Resource Data Name` :type Name))
  (bind _resourcedata_name (break `/Game/Blueprints/Structures/STRUCT_ResourceData` (`self.ResourceData`)))
  (return _resourcedata_name))

(fn `UserConstructionScript`
  (bind (_name _type _mesh _soundongrabbed) (break `/Game/Blueprints/Structures/STRUCT_ResourceData` (`self.ResourceData`)))
  (`parent.UserConstructionScript`)
  (bind _returnvalue (`|GetDataTableRow` "/Game/Blueprints/DataTables/DT_Resources.DT_Resources" (`self.DT_Row`))
    (:`then`
      (set `self.ResourceData` _returnvalue)
      (`StaticMeshComponent.SetStaticMesh` (`self.StaticMesh`) _mesh)
      (set `self.Sound_OnGrabbed` _soundongrabbed))))