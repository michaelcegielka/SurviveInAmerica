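; BP_ConstructionSlot is a slot that a matching BP_Resource snaps into, previewed by a display mesh set in the construction script.
; On collision overlap, it compares the resource's name to ResourceName and tries to release whatever the player pawn holds in its right hand.
; If the release succeeds, it teleports the resource to the preview mesh's transform, clears that mesh and marks the slot as used.
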(event `self.Collision.OnComponentBeginOverlap`
  (params (OverlappedComponent :type "PrimitiveComponent Object Reference") (OtherActor :type "Actor Object Reference") (OtherComp :type "PrimitiveComponent Object Reference") (OtherBodyIndex :type Integer) (bFromSweep :type Boolean) (SweepResult :type "HitResult Structure (by ref)"))
  (bind _asbp_resource (cast `/Game/Blueprints/Items/BP_Resource` OtherActor))
  (if (== (`self.ResourceName`) (`/Game/Blueprints/Items/BP_Resource.GetName` _asbp_resource))
    (bind _asbp_player_pawn (cast `/Game/Blueprints/Player/BP_PlayerPawn` (`GameplayStatics.GetPlayerPawn` 0)))
    (bind _heldcomponentright (`/Game/Blueprints/Player/BP_PlayerPawn.HeldComponentRight` _asbp_player_pawn))
    (if (`KismetSystemLibrary.IsValid` _heldcomponentright)
      (bind _breleased (`/Game/Blueprints/Interactables/BP_GrabComponent.TryRelease` _heldcomponentright))
      (if _breleased
        (`self.K2_SetActorTransform` _asbp_resource (`SceneComponent.K2_GetComponentToWorld` (`self.StaticMesh`)) false true)
        (`StaticMeshComponent.SetStaticMesh` (`self.StaticMesh`) null)
        (set `self.Used` true)))))

(fn `UserConstructionScript`
  (`StaticMeshComponent.SetStaticMesh` (`self.StaticMesh`) (`self.DisplayMesh`)))