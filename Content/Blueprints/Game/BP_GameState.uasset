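; Game State Blueprint that stores a match countdown as TimerMinutes and TimerSeconds and exposes it through getters and setters.
; GetTime returns both values plus a "TIME_LEFT :" display string, branching to zero-pad minutes and seconds below ten and rounding each value.
; It does not advance the timer itself, as the event graph holds only disabled placeholder events.
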(fn `GetTime`
  (returns (TimerMinutes :type "Float (double-precision)") (TimerSeconds :type "Float (double-precision)") (String :type String))
  (bind _timerseconds (`self.GetTimerSeconds`))
  (bind _timerseconds_2 (`self.GetTimerSeconds`))
  (bind _returnvalue (`KismetStringLibrary.Conv_Int64ToString` (`KismetMathLibrary.Round64` _timerseconds_2)))
  (bind _returnvalue_2 (`KismetStringLibrary.Conv_Int64ToString` (`KismetMathLibrary.Round64` _timerseconds)))
  (bind _returnvalue_3 (`KismetStringLibrary.Concat_StrStr` (`KismetStringLibrary.Concat_StrStr` "TIME_LEFT :  " (`KismetStringLibrary.Conv_Int64ToString` (`KismetMathLibrary.Round64` (`self.GetTimerMinutes`)))) " : "))
  (bind _returnvalue_4 (`KismetStringLibrary.Concat_StrStr` (`KismetStringLibrary.Concat_StrStr` (`KismetStringLibrary.Concat_StrStr` "TIME_LEFT :  " "0") (`KismetStringLibrary.Conv_Int64ToString` (`KismetMathLibrary.Round64` (`self.GetTimerMinutes`)))) " : "))
  (if (< (`self.GetTimerMinutes`) 10.0)
    (if (< _timerseconds_2 10.0)
      (return (`self.GetTimerMinutes`) (`self.GetTimerSeconds`) (`KismetStringLibrary.Concat_StrStr` (`KismetStringLibrary.Concat_StrStr` _returnvalue_4 "0") _returnvalue))
      (else
        (return (`self.GetTimerMinutes`) (`self.GetTimerSeconds`) (`KismetStringLibrary.Concat_StrStr` _returnvalue_4 _returnvalue))))
    (elif (< _timerseconds 10.0)
      (return (`self.GetTimerMinutes`) (`self.GetTimerSeconds`) (`KismetStringLibrary.Concat_StrStr` (`KismetStringLibrary.Concat_StrStr` _returnvalue_3 "0") _returnvalue_2))
      (else
        (return (`self.GetTimerMinutes`) (`self.GetTimerSeconds`) (`KismetStringLibrary.Concat_StrStr` _returnvalue_3 _returnvalue_2))))))

(fn `GetTimerMinutes`
  (returns (TimerMinutes :type "Float (double-precision)"))
  (return (`self.TimerMinutes`)))

(fn `GetTimerSeconds`
  (returns (TimerSeconds :type "Float (double-precision)"))
  (return (`self.TimerSeconds`)))

(fn `SetTimerMinutes`
  (params (NewTimerMinutes :type "Float (double-precision)"))
  (set `self.TimerMinutes` NewTimerMinutes))

(fn `SetTimerSeconds`
  (params (NewTimerSeconds :type "Float (double-precision)"))
  (set `self.TimerSeconds` NewTimerSeconds))

(fn `UserConstructionScript`)