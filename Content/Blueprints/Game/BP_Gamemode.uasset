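; Game mode that runs the match countdown, storing minutes and seconds in BP_GameState.
; BeginPlay caches the game state and calls StartGame, which opens a Tick gate feeding ReduceGameTime.
; Each tick subtracts a fixed step independent of delta time, rolling minutes over and firing the empty MinutePassed event.
; When minutes run out, it closes the gate and calls EndGame as unsuccessful, though EndGame is still a stub.
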(event `self.ReceiveBeginPlay`
  (set `self.BP_GameState_ref` (cast `/Game/Blueprints/Game/BP_GameState` (`GameplayStatics.GetGameState`) :!pure true))
  (`self.StartGame`))

(event `self.ReceiveTick`
  (params (DeltaSeconds :type "Float (single-precision)"))
  (`/Engine/EditorBlueprintResources/StandardMacros.Gate` true :!label _label
    (:`Exit`
      (`self.Reduce Game Time` 1.0))))

(event `OpenTickGate`
  (goto _label :!via `Open`))

(event `CloseTickGate`
  (goto _label :!via `Close`))

(event `MinutePassed`)

(fn `EndGame`
  (params (`Sucessfull?` :type Boolean)))

(fn `Reduce Game Time`
  (params (Scale :type "Float (double-precision)" :default 1.0))
  (bind _bp_gamestate_ref (`self.BP_GameState_ref`))
  (bind _returnvalue (- (`.TimerSeconds` (`/Game/Blueprints/Game/BP_GameState.GetTime` (`self.BP_GameState_ref`))) (* Scale 0.02)))
  (bind _returnvalue_2 (- (`/Game/Blueprints/Game/BP_GameState.GetTimerMinutes` _bp_gamestate_ref) 1.0))
  (if (<= _returnvalue 0.0)
    (`/Game/Blueprints/Game/BP_GameState.SetTimerSeconds` _bp_gamestate_ref 59.59)
    (if (< _returnvalue_2 0.0)
      (`self.CloseTickGate`)
      (`self.EndGame` false)
      (else
        (`/Game/Blueprints/Game/BP_GameState.SetTimerMinutes` (`self.BP_GameState_ref`) _returnvalue_2)
        (`self.MinutePassed`)))
    (else
      (`/Game/Blueprints/Game/BP_GameState.SetTimerSeconds` (`self.BP_GameState_ref`) _returnvalue))))

(fn `StartGame`
  (`self.OpenTickGate`))

(fn `UserConstructionScript`)